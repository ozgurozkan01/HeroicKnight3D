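; BP_MainPlayerController is a player controller that adds animated transitions to showing and removing the pause menu.
; It extends the parent's display and remove events, casting the PauseMenu widget to PauseMenuHUD to play PauseMenuAnimation forward on open and in reverse on close.
; On close, a short fixed delay, rather than an animation-finished callback, precedes hiding the widget.
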(event `self.DisplayPauseMenu`
  (`parent.DisplayPauseMenu`)
  (bind _aspause_menu_hud (cast `/Game/HUD/PauseMenuHUD` (`self.PauseMenu`)))
  (`UserWidget.PlayAnimation` _aspause_menu_hud (`/Game/HUD/PauseMenuHUD.PauseMenuAnimation` _aspause_menu_hud) 0.0 1 "Forward" 1.0 false))

(event `self.RemovePauseMenu`
  (`parent.RemovePauseMenu`)
  (bind _aspause_menu_hud (cast `/Game/HUD/PauseMenuHUD` (`self.PauseMenu`)))
  (`UserWidget.PlayAnimation` _aspause_menu_hud (`/Game/HUD/PauseMenuHUD.PauseMenuAnimation` _aspause_menu_hud) 0.0 1 "Reverse" 1.0 false)
  (`KismetSystemLibrary.Delay` 0.4)
  (`Widget.SetVisibility` (`self.PauseMenu`) "Hidden"))

(fn `UserConstructionScript`)